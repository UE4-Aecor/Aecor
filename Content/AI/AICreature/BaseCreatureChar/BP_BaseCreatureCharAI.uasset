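; Base creature AI character Blueprint that provides a custom movement input event which turns the creature as it moves.
; AddMovementInputCustom smoothly interpolates actor rotation toward the world direction, clamping pitch and roll to a narrow range while yaw stays free.
; It then passes the direction and scale to standard AddMovementInput, and the construction script is empty.
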(event `self.AddMovementInputCustom`
  (params (WorldDirection :type "Vector Structure") (ScaleValue :type "Float (single-precision)"))
  (`self.K2_SetActorRotation` (`KismetMathLibrary.RInterpTo` (`self.K2_GetActorRotation`) (`KismetMathLibrary.MakeRotator` (`KismetMathLibrary.FClamp` (.roll (`KismetMathLibrary.MakeRotFromX` WorldDirection)) -10.0 10.0) (`KismetMathLibrary.FClamp` (.pitch (`KismetMathLibrary.MakeRotFromX` WorldDirection)) -10.0 10.0) (.yaw (`KismetMathLibrary.MakeRotFromX` WorldDirection))) (`GameplayStatics.GetWorldDeltaSeconds`) 5.0))
  (`self.AddMovementInput` WorldDirection (* ScaleValue 1.0)))

(fn `UserConstructionScript`)