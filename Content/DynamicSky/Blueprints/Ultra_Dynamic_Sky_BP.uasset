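; Dynamic sky actor that drives a day/night cycle with sun, moon phases, stars, auroras and changing cloud cover.
; Tick advances TimeOfDay, uses Delays to retarget cloud density, step moon phase and recapture the skylight.
; SetSolarAngle rotates sun and moon.
; SetMaterialVariables feeds sky, moon and cloud-shadow light-function materials, coloring lights, fog and optional fast skylight from time-of-day curves or manual values.
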(event `self.ReceiveTick`
  (params (DeltaSeconds :type "Float (single-precision)"))
  (bind _skylight (`self.Skylight`))
  (bind _returnvalue (+ (`self.Moon Phase`) 1.0))
  (bind _returnvalue_2 (+ (`self.Time of Day`) (/ (* (/ DeltaSeconds 60.0) 2400.0) (`self.Day Length`))))
  (`|ExecutionSequence`
    (:`then_0`
      ;[1 1 1] Dynamic Cloud Weather
      (if (`self.Simulate Cloud Density Changes`)
        (`KismetSystemLibrary.Delay` (`KismetMathLibrary.RandomFloatInRange` (* (`self.Cloud Density Shift Frequency (min)`) 60.0) (* (`self.Cloud Density Shift Frequency (max)`) 60.0)))
        (set `self.Cloud Density_target` (`KismetMathLibrary.RandomFloatInRange` 0.0 3.6))))
    (:`then_1`
      ;[1 1 1] Day/Night Cycle
      (if (`self.Animate Day/Night Cycle`)
        (set `self.Time of Day` (`KismetMathLibrary.SelectFloat` 2400.0 (`KismetMathLibrary.SelectFloat` 0.0 _returnvalue_2 (> _returnvalue_2 2400.0)) (< _returnvalue_2 0.0))))
      (`self.Set Solar Angle`))
    (:`then_2`
      ;[1 1 1] Animate Cloud Density
      (if (`self.Simulate Cloud Density Changes`)
        (set `self.Cloud Density` (`KismetMathLibrary.Lerp` (`self.Cloud Density`) (`self.Cloud Density_target`) (/ (`self.Cloud Density Change (Smoothing)`) 5.0)))))
    (:`then_3`
      (`self.Set Material Variables`))
    (:`then_4`
      ;[1 1 1] Lunar Phase Simulation
      (if (`self.Simulate Moon Phase Changes`)
        (if (`self.First Day`)
          (`KismetSystemLibrary.Delay` (- 2400.0 (`self.Time of Day`)))
          (set `self.First Day` false))
        (`KismetSystemLibrary.Delay` (* (`self.Day Length`) 60.0))
        (set `self.Moon Phase` (`KismetMathLibrary.SelectFloat` 27.0 (`KismetMathLibrary.SelectFloat` 0.0 _returnvalue (> _returnvalue 27.0)) (< _returnvalue 0.0)))))
    (:`then_5`
      ;[1 1 1] Recapture Skylight
      (if (and (`self.Recapture Sky light periodically`) (`self.Animate Day/Night Cycle`) (not (`self.Use Fast Skylight`)))
        (`KismetSystemLibrary.Delay` (`self.Sky Light recapture period`))
        (if (`KismetSystemLibrary.IsValid` _skylight)
          (`SkyLightComponent.RecaptureSky` (`SkyLight.LightComponent` _skylight)))))))

(event `self.ReceiveBeginPlay`
  ;[1 1 1] Equalize Cloud Density Delta
  (set `self.Cloud Density_target` (`self.Cloud Density`)))

(fn `Set Material Variables`
  (bind _output_color (`self.Adjust color for night brightness` (struct :`R` 0.305882 :`G` 0.333333 :`B` 0.372549 :`A` 1.0)))
  (bind _udm_mat (`self.UDM_mat`))
  (bind _direction_light__sun_ (`self.Direction Light (Sun)`))
  (bind _direction_light__sun__2 (`self.Direction Light (Sun)`))
  (bind _exponential_height_fog (`self.Exponential Height Fog`))
  (bind _horizon_base_color (`self.Horizon Base Color`))
  (bind _udm_mat_2 (`self.UDM_mat`))
  (bind _direction_light__sun__3 (`self.Direction Light (Sun)`))
  (bind _sun_light_color (`self.Sun Light Color`))
  (bind _moon_light (`self.Moon Light`))
  (bind _clouds_base_texture (`self.Clouds Base Texture`))
  (bind _moon_light_2 (`self.Moon Light`))
  (bind _time_of_day (`self.Time of Day`))
  (bind _udm_mat_3 (`self.UDM_mat`))
  (bind _sun_rotation (`self.Sun Rotation`))
  (bind _direction_light__sun__4 (`self.Direction Light (Sun)`))
  (bind _exponential_height_fog_2 (`self.Exponential Height Fog`))
  (bind _cloud_shadows_scale (`self.Cloud Shadows Scale`))
  (bind _cloud_shadows_mid (`self.Cloud Shadows MID`))
  (bind _returnvalue (`KismetMathLibrary.MapRangeUnclamped` (`self.Sun Inclination`) 0.0 90.0 0.0 1.0))
  (bind _returnvalue_2 (- (`self.color_scheme`) 1))
  (bind _returnvalue_3 (select `bool` (`self.Use Cloud Shadows`) :`true` (`self.Cloud Shadows MID`) :!type "MaterialInterface Object Reference"))
  (bind _lightcomponent (`Light.LightComponent` _direction_light__sun__2))
  (bind _component (`ExponentialHeightFog.Component` _exponential_height_fog))
  (bind _lightcomponent_2 (`Light.LightComponent` _moon_light))
  (bind _lightcomponent_3 (`Light.LightComponent` _moon_light_2))
  (bind _lightcomponent_4 (`Light.LightComponent` _direction_light__sun__4))
  (bind _lightcomponent_5 (`SkyLight.LightComponent` (`self.Skylight`)))
  (bind _returnvalue_4 (`KismetMathLibrary.FClamp` (`KismetMathLibrary.MapRangeUnclamped` (`self.Cloud Density`) 2.0 2.5 0.0 1.0) 0.0 0.8))
  (bind _z (.z (`self.GetActorForwardVector` _moon_light)))
  (bind _z_2 (.z (`self.GetActorForwardVector` _direction_light__sun__2)))
  (bind _returnvalue_5 (`KismetMathLibrary.SelectFloat` (`KismetMathLibrary.Lerp` (`KismetMathLibrary.MapRangeUnclamped` _time_of_day 0.0 1200.0 0.0 1.0) 0.5 _returnvalue) (`KismetMathLibrary.Lerp` (`KismetMathLibrary.MapRangeUnclamped` _time_of_day 1200.0 2400.0 1.0 0.0) 0.5 _returnvalue) (< _time_of_day 1200.0)))
  (bind _returnvalue_6 (`CurveLinearColor.GetLinearColorValue` (`|GetArrayItem` (`self.Sun Color Curve`) _returnvalue_2) _returnvalue_5))
  (bind _returnvalue_7 (`CurveLinearColor.GetLinearColorValue` (`|GetArrayItem` (`self.Horizon Base Color Curve`) _returnvalue_2) _returnvalue_5))
  (bind _returnvalue_8 (`CurveLinearColor.GetLinearColorValue` (`|GetArrayItem` (`self.Zenith Base Color Curve`) _returnvalue_2) _returnvalue_5))
  (bind _returnvalue_9 (`CurveFloat.GetFloatValue` (`self.Stars Intensity Curve`) _returnvalue_5))
  (bind _output_color_2 (`self.Adjust color for night brightness` _returnvalue_7))
  (bind _output_color_3 (`self.Adjust color for night brightness` _returnvalue_8))
  (bind _returnvalue_10 (`KismetMathLibrary.LinearColorLerp` _output_color_2 _output_color _returnvalue_4))
  (bind _returnvalue_11 (select `bool` (`self.Manually Select Sun Color`) :`false` (`KismetMathLibrary.LinearColorLerp` _returnvalue_6 (`CurveLinearColor.GetLinearColorValue` (`self.Sun Cloudy Color Curve`) _returnvalue_5) _returnvalue_4) :`true` (`self.Sun Color`)))
  (if (`KismetSystemLibrary.IsValid` _direction_light__sun_)
    ;[1 1 1] Set Material Parameters
    (`MaterialInstanceDynamic.SetVectorParameterValue` _udm_mat "Sun Position" (`KismetMathLibrary.Conv_VectorToLinearColor` (`KismetMathLibrary.Conv_RotatorToVector` (`self.K2_GetActorRotation` _direction_light__sun_))))
    (set `self.Sun Yaw` (.yaw (`SceneComponent.K2_GetComponentRotation` (`Light.LightComponent` _direction_light__sun_))))
    (else
      (`MaterialInstanceDynamic.SetVectorParameterValue` _udm_mat "Sun Position" (`KismetMathLibrary.Conv_VectorToLinearColor` (`KismetMathLibrary.Conv_RotatorToVector` _sun_rotation)))
      (set `self.Sun Yaw` (.yaw _sun_rotation))))
  (`MaterialInstanceDynamic.SetVectorParameterValue` _udm_mat "Moon Light Vector" (`KismetMathLibrary.Conv_VectorToLinearColor` (`KismetMathLibrary.Conv_RotatorToVector` (`SceneComponent.K2_GetComponentRotation` (`self.Arrow`)))))
  (`MaterialInstanceDynamic.SetScalarParameterValue` _udm_mat "Cloud Speed" (`self.Cloud Speed`))
  (`MaterialInstanceDynamic.SetScalarParameterValue` (`self.Cloud Shadows MID`) "Cloud Speed" (`self.Cloud Speed`))
  (`MaterialInstanceDynamic.SetScalarParameterValue` _udm_mat "Cloud Density" (`self.Cloud Density`))
  (`MaterialInstanceDynamic.SetScalarParameterValue` (`self.Cloud Shadows MID`) "Cloud Density" (`self.Cloud Density`))
  (`MaterialInstanceDynamic.SetScalarParameterValue` _udm_mat "Wispy Cloud Alpha" (`self.Cloud Wisps Opacity`))
  (`MaterialInstanceDynamic.SetScalarParameterValue` _udm_mat "Cloud Phase" (`self.Cloud Phase`))
  (`MaterialInstanceDynamic.SetScalarParameterValue` (`self.Cloud Shadows MID`) "Cloud Phase" (`self.Cloud Phase`))
  (`MaterialInstanceDynamic.SetScalarParameterValue` _udm_mat "Moon Scale" (`self.Moon Scale`))
  (`MaterialInstanceDynamic.SetScalarParameterValue` _udm_mat "Lunar Inclination" (`self.Moon Inclination`))
  (`MaterialInstanceDynamic.SetScalarParameterValue` _udm_mat "Lunar Phase" (`KismetMathLibrary.Conv_IntToDouble` (`KismetMathLibrary.Round` (`self.Moon Phase`))))
  (`MaterialInstanceDynamic.SetScalarParameterValue` (`self.Moon mat`) "Lunar Phase" (`KismetMathLibrary.Conv_IntToDouble` (`KismetMathLibrary.Round` (`self.Moon Phase`))))
  (`MaterialInstanceDynamic.SetScalarParameterValue` _udm_mat "Moon Intensity" (`self.Moon Intensity`))
  (`MaterialInstanceDynamic.SetScalarParameterValue` (`self.Moon mat`) "Moon Intensity" (`self.Moon Intensity`))
  (`MaterialInstanceDynamic.SetScalarParameterValue` _udm_mat "Cloud Opacity" (`self.Cloud Opacity`))
  (`MaterialInstanceDynamic.SetScalarParameterValue` _udm_mat "Saturation" (`self.Saturation`))
  (`MaterialInstanceDynamic.SetScalarParameterValue` _udm_mat "Overall Intensity" (`self.Overall Intensity`))
  (`MaterialInstanceDynamic.SetScalarParameterValue` _udm_mat "Sun Brightness" (`self.Sun Brightness`))
  (`MaterialInstanceDynamic.SetVectorParameterValue` _udm_mat "Moon Color" (`self.Moon Color`))
  (`MaterialInstanceDynamic.SetVectorParameterValue` (`self.Moon mat`) "Moon Color" (`self.Moon Color`))
  (`MaterialInstanceDynamic.SetScalarParameterValue` _udm_mat "Shine Variation" (`self.Shine Variation`))
  (`MaterialInstanceDynamic.SetScalarParameterValue` _udm_mat "Sun Lighting Intensity" (`self.Sun Lighting Intensity`))
  (`MaterialInstanceDynamic.SetVectorParameterValue` _udm_mat "Stars Color" (`self.Stars_Color`))
  (`MaterialInstanceDynamic.SetScalarParameterValue` _udm_mat "Moon Cycle Offset" (`self.Moon Orbit Offset`))
  (`MaterialInstanceDynamic.SetScalarParameterValue` _udm_mat "Sun Radius" (`self.Sun Radius`))
  (`MaterialInstanceDynamic.SetScalarParameterValue` _udm_mat "Stars Speed" (`self.Stars Speed`))
  (`MaterialInstanceDynamic.SetScalarParameterValue` _udm_mat "Moon Rotation" (`self.Moon Rotation`))
  (`MaterialInstanceDynamic.SetTextureParameterValue` _udm_mat "CustomMoonTexture" (`self.Custom Moon Texture`))
  (`MaterialInstanceDynamic.SetTextureParameterValue` (`self.Moon mat`) "CustomMoonTexture" (`self.Custom Moon Texture`))
  (`MaterialInstanceDynamic.SetScalarParameterValue` _udm_mat "UseCustomMoonTexture" (`KismetMathLibrary.SelectFloat` 1.0 0.0 (`self.Use Custom Moon Texture`)))
  (`MaterialInstanceDynamic.SetScalarParameterValue` (`self.Moon mat`) "UseCustomMoonTexture" (`KismetMathLibrary.SelectFloat` 1.0 0.0 (`self.Use Custom Moon Texture`)))
  (`MaterialInstanceDynamic.SetScalarParameterValue` _udm_mat "Moon Glow Intensity" (`self.Moon Glow Intensity`))
  (`MaterialInstanceDynamic.SetTextureParameterValue` _udm_mat "clouds_basetex" _clouds_base_texture)
  (`MaterialInstanceDynamic.SetScalarParameterValue` _udm_mat "Cloud Tiling" (`self.Cloud Tiling`))
  (`MaterialInstanceDynamic.SetScalarParameterValue` _udm_mat "Cloud Direction" (`self.Cloud Direction`))
  (`MaterialInstanceDynamic.SetScalarParameterValue` _udm_mat "Cloud Height 1" (`KismetMathLibrary.MapRangeUnclamped` (`self.Cloud Height 1`) 1.0 0.0 0.0 0.8))
  (`MaterialInstanceDynamic.SetScalarParameterValue` _udm_mat "Cloud Height 2" (`KismetMathLibrary.MapRangeUnclamped` (`self.Cloud Height 2`) 1.0 0.0 0.0 0.8))
  (`MaterialInstanceDynamic.SetTextureParameterValue` _cloud_shadows_mid "clouds_basetex" _clouds_base_texture)
  (`MaterialInstanceDynamic.SetScalarParameterValue` _cloud_shadows_mid "Shadows Intensity" (`self.Cloud Shadows Intensity`))
  (`MaterialInstanceDynamic.SetScalarParameterValue` _cloud_shadows_mid "Shadows Scale" (`self.Cloud Shadows Scale`))
  (`MaterialInstanceDynamic.SetScalarParameterValue` _cloud_shadows_mid "Sun Yaw" (`self.Sun Yaw`))
  (`MaterialInstanceDynamic.SetScalarParameterValue` _cloud_shadows_mid "rotation" (+ (* (/ (.yaw (`self.K2_GetActorRotation`)) 360.0) -1.0) (`self.Cloud Direction`)))
  ;[1 1 1] Setting Cloud Shadows
  (`MaterialInstanceDynamic.SetScalarParameterValue` _cloud_shadows_mid "One cloud layer" (select `bool` (`self.One Cloud Layer`) :`false` 1.0 :`true` 0.0 :!type "Float (single-precision)"))
  (if (`KismetSystemLibrary.IsValid` _direction_light__sun__3)
    (`LightComponent.SetLightFunctionMaterial` (`Light.LightComponent` _direction_light__sun__3) _returnvalue_3))
  (if (`KismetSystemLibrary.IsValid` _moon_light_2)
    (`LightComponent.SetLightFunctionMaterial` _lightcomponent_3 _returnvalue_3)
    (`LightComponent.SetLightFunctionScale` _lightcomponent_3 (`KismetMathLibrary.MakeVector` _cloud_shadows_scale _cloud_shadows_scale _cloud_shadows_scale)))
  (if (`self.Automatically Set Advanced Settings using Time of Day`)
    ;[1 1 1] Automatic Entry of Advanced Variables
    (`MaterialInstanceDynamic.SetVectorParameterValue` _udm_mat_2 "Horizon Base Color" _output_color_2)
    (`MaterialInstanceDynamic.SetVectorParameterValue` _udm_mat_2 "Zenith Base Color" _output_color_3)
    (`MaterialInstanceDynamic.SetVectorParameterValue` _udm_mat_2 "Cloud Light Color" (`self.Adjust color for night brightness` (`CurveLinearColor.GetLinearColorValue` (`|GetArrayItem` (`self.Cloud Light Color Curve`) _returnvalue_2) _returnvalue_5)))
    (`MaterialInstanceDynamic.SetVectorParameterValue` _udm_mat_2 "Cloud Dark Color" (`self.Adjust color for night brightness` (`CurveLinearColor.GetLinearColorValue` (`|GetArrayItem` (`self.Cloud Dark Color Curve`) _returnvalue_2) _returnvalue_5)))
    (`MaterialInstanceDynamic.SetVectorParameterValue` _udm_mat_2 "Sun Color" _returnvalue_6)
    (`MaterialInstanceDynamic.SetScalarParameterValue` _udm_mat_2 "Shine Intensity" (`CurveFloat.GetFloatValue` (`self.Shine Intensity Curve`) _returnvalue_5))
    (`MaterialInstanceDynamic.SetScalarParameterValue` _udm_mat_2 "Moon Position" (`CurveFloat.GetFloatValue` (`self.Moon Position Curve`) (`KismetMathLibrary.MapRangeUnclamped` (`self.Time of Day`) 0.0 2400.0 0.0 1.0)))
    (`MaterialInstanceDynamic.SetScalarParameterValue` _udm_mat_2 "Sun Highlight Radius" (`CurveFloat.GetFloatValue` (`self.Sun Highlight Radius_curve`) _returnvalue_5))
    (`MaterialInstanceDynamic.SetScalarParameterValue` _udm_mat_2 "Stars Intensity" (* _returnvalue_9 (`self.Stars_Intensity`)))
    (`MaterialInstanceDynamic.SetScalarParameterValue` _udm_mat_2 "Aurora Intensity" (* _returnvalue_9 (/ (`self.Aurora Intensity`) 15.0)))
    (`MaterialInstanceDynamic.SetScalarParameterValue` _udm_mat_2 "Aurora Speed" (`self.Aurora Speed`))
    (if (`KismetSystemLibrary.IsValid` _direction_light__sun__2)
      (`LightComponent.SetLightColor` _lightcomponent _returnvalue_11 true)
      (`LightComponent.SetBloomTint` _lightcomponent (`KismetMathLibrary.Conv_LinearColorToColor` _returnvalue_11))
      (`ActorComponent.SetActive` _lightcomponent (> _z_2 0.0) false)
      (`LightComponent.SetIntensity` _lightcomponent (* (`CurveFloat.GetFloatValue` (`self.Directional_Intensity_Curve`) _z_2) (`self.Sun_Light_Intensity`)))
      (`LightComponent.SetVolumetricScatteringIntensity` _lightcomponent (`KismetMathLibrary.MapRangeClamped` (`KismetMathLibrary.MultiplyMultiply_FloatFloat` (`KismetMathLibrary.MapRangeClamped` (`self.Cloud Density`) 0.0 2.1 0.0 1.0) 0.5) 0.0 1.0 (`self.Sun_Volumetric_Scattering_Intensity`))))
    (if (`KismetSystemLibrary.IsValid` _exponential_height_fog)
      (`ExponentialHeightFogComponent.SetFogInscatteringColor` _component (`KismetMathLibrary.LinearColorLerp` _output_color_2 (`KismetMathLibrary.LinearColorLerp` _output_color_2 _output_color_2 0.4) _returnvalue_4))
      (`ExponentialHeightFogComponent.SetDirectionalInscatteringColor` _component _returnvalue_10))
    (if (`KismetSystemLibrary.IsValid` _moon_light)
      (`LightComponent.SetLightColor` _lightcomponent_2 (`self.Adjust color for night brightness` (`self.Moon Color`)) true)
      (`LightComponent.SetIntensity` _lightcomponent_2 (* (`CurveFloat.GetFloatValue` (`self.Directional_Intensity_Curve`) _z) (`self.Moonlight Intensity`)))
      (`ActorComponent.SetActive` _lightcomponent_2 (> _z 0.0) false)
      (`LightComponent.SetVolumetricScatteringIntensity` _lightcomponent_2 (`KismetMathLibrary.MapRangeClamped` (`KismetMathLibrary.MultiplyMultiply_FloatFloat` (`KismetMathLibrary.MapRangeClamped` (`self.Cloud Density`) 0.0 2.1 0.0 1.0) 0.5) 0.0 1.0 (`self.Moon_Volumetric_Scattering_Intensity`))))
    (`/Engine/EditorBlueprintResources/StandardMacros.IsValid` (`self.Skylight`)
      (:`Is Valid`
        (if (`self.Use Fast Skylight`)
          (`SkyLightComponent.SetLightColor` _lightcomponent_5 (`KismetMathLibrary.LinearColorLerp` (`KismetMathLibrary.LinearColorLerp` (`KismetMathLibrary.LinearColorLerp` (`KismetMathLibrary.LinearColorLerp` _returnvalue_7 _output_color _returnvalue_4) (`KismetMathLibrary.LinearColorLerp` _returnvalue_8 _output_color _returnvalue_4) 0.0) (`KismetMathLibrary.LinearColorLerp` (`KismetMathLibrary.LinearColorLerp` _output_color_3 _output_color _returnvalue_4) _returnvalue_10 0.0) 0.8) (`self.Adjust color for night brightness` (struct :`R` 1.0 :`G` 1.0 :`B` 1.0 :`A` 1.0)) 0.2))
          (else
            (`SkyLightComponent.SetLightColor` _lightcomponent_5 (struct :`R` 1.0 :`G` 1.0 :`B` 1.0 :`A` 1.0))))))
    (else
      ;[1 1 1] Manual Entry of Advanced Variables
      (`MaterialInstanceDynamic.SetVectorParameterValue` _udm_mat_3 "Horizon Base Color" _horizon_base_color)
      (`MaterialInstanceDynamic.SetVectorParameterValue` _udm_mat_3 "Zenith Base Color" (`self.Zenith Base Color`))
      (`MaterialInstanceDynamic.SetVectorParameterValue` _udm_mat_3 "Cloud Light Color" (`self.Cloud Light Color`))
      (`MaterialInstanceDynamic.SetVectorParameterValue` _udm_mat_3 "Cloud Dark Color" (`self.Cloud Dark Color`))
      (`MaterialInstanceDynamic.SetVectorParameterValue` _udm_mat_3 "Sun Color" (`self.Sun Color`))
      (`MaterialInstanceDynamic.SetScalarParameterValue` _udm_mat_3 "Shine Intensity" (`self.Cloud Shine Intensity`))
      (`MaterialInstanceDynamic.SetScalarParameterValue` _udm_mat_3 "Stars Intensity" (* (`self.Stars Visibility`) (`self.Stars_Intensity`)))
      (`MaterialInstanceDynamic.SetScalarParameterValue` _udm_mat_3 "Moon Position" (`self.Moon Position`))
      (`MaterialInstanceDynamic.SetScalarParameterValue` _udm_mat_3 "Sun Highlight Radius" (`self.Sun Highlight Radius`))
      (if (`KismetSystemLibrary.IsValid` _direction_light__sun__4)
        (`LightComponent.SetLightColor` _lightcomponent_4 _sun_light_color true)
        (`LightComponent.SetBloomTint` _lightcomponent_4 (`KismetMathLibrary.Conv_LinearColorToColor` _sun_light_color)))
      (if (`KismetSystemLibrary.IsValid` _exponential_height_fog_2)
        (`ExponentialHeightFogComponent.SetFogInscatteringColor` (`ExponentialHeightFog.Component` _exponential_height_fog_2) _horizon_base_color)))))

(fn `Set Solar Angle`
  (bind _sun_root (`self.Sun_Root`))
  (bind _direction_light__sun_ (`self.Direction Light (Sun)`))
  (bind _moon_plane (`self.moon_plane`))
  (bind _returnvalue (+ (`CurveFloat.GetFloatValue` (`self.Moon Position Curve`) (`KismetMathLibrary.MapRangeUnclamped` (`self.Time of Day`) 0.0 2400.0 0.0 1.0)) (`self.Moon Orbit Offset`)))
  ;[1 1 1] Set Directional Light Rotation
  (`SceneComponent.K2_SetWorldRotation` _sun_root (`KismetMathLibrary.Conv_VectorToRotator` (`KismetMathLibrary.GreaterGreater_VectorRotator` (`KismetMathLibrary.GetAxes` (`KismetMathLibrary.MakeRotator` 0.0 0.0 (`self.Sun Inclination`))) (`KismetMathLibrary.MakeRotator` 0.0 (+ (`KismetMathLibrary.MapRangeUnclamped` (`self.Time of Day`) 0.0 2400.0 0.0 360.0) 90.0) (`self.Sun Angle`)))) false false)
  (if (and (`KismetSystemLibrary.IsValid` _direction_light__sun_) (`self.Automatically Set Sun Light Rotation`))
    (`self.K2_SetActorRotation` _direction_light__sun_ (`SceneComponent.K2_GetComponentRotation` _sun_root) false))
  ;[1 1 1] Set Moonlight Angle
  (`SceneComponent.K2_SetWorldRotation` (`self.Arrow`) (`KismetMathLibrary.MakeRotFromXY` (`KismetMathLibrary.GreaterGreater_VectorRotator` (`KismetMathLibrary.GreaterGreater_VectorRotator` (`KismetMathLibrary.GetAxes` (`KismetMathLibrary.MakeRotator` 0.0 0.0 (* (`self.Moon Inclination`) 131.4))) (`KismetMathLibrary.MakeRotator` 0.0 (* (+ (* (- (- _returnvalue (`KismetMathLibrary.Conv_IntToDouble` (`KismetMathLibrary.FFloor` _returnvalue))) 0.5) 2.179) 0.5) -180.0))) (`KismetMathLibrary.MakeRotator` 0.0 0.0 (`self.Moon Angle`))) (`KismetMathLibrary.MakeVector` 0.0 1.0 0.0)) false false)
  (`SceneComponent.SetRelativeScale3D` _moon_plane (`KismetMathLibrary.Conv_DoubleToVector` (* (`self.Moon Scale`) 10400.0)))
  (`SceneComponent.K2_SetRelativeRotation` _moon_plane (`KismetMathLibrary.MakeRotator` (`self.Moon Rotation`)) false false)
  (if (and (`KismetSystemLibrary.IsValid` (`self.Moon Light`)) (`self.Automatically Set Moon Light Rotation`))
    (`self.K2_SetActorRotation` (`self.Moon Light`) (`SceneComponent.K2_GetComponentRotation` (`self.Arrow`)) false)))

(fn `UserConstructionScript`
  (bind _skylight (`self.Skylight`))
  (bind _use_auroras (`self.Use Auroras`))
  (bind _returnvalue (`KismetMaterialLibrary.CreateDynamicMaterialInstance` "/Game/DynamicSky/Materials/Cloud_Shadows.Cloud_Shadows"))
  (set `self.Cloud Shadows MID` _returnvalue)
  (if (`self.Refresh Settings`)
    _
    (else
      _))
  (set `self.Refresh Settings` false) ; Use the refresh settings variable to reset settings
  (bind _returnvalue_2 (`PrimitiveComponent.CreateDynamicMaterialInstance` (`self.Ultra_Dynamic_Sky_Sphere`) 0 (select `bool` (`self.One Cloud Layer`) :`false` (select `bool` _use_auroras :`false` "/Game/DynamicSky/Materials/Ultra_Dynamic_Sky_Mat_no_auroras.Ultra_Dynamic_Sky_Mat_no_auroras" :`true` "/Game/DynamicSky/Materials/Ultra_Dynamic_Sky_Mat.Ultra_Dynamic_Sky_Mat" :!type "MaterialInterface Object Reference") :`true` (select `bool` _use_auroras :`false` "/Game/DynamicSky/Materials/Ultra_Dynamic_Sky_Mat_no_auroras_onecloudlayer.Ultra_Dynamic_Sky_Mat_no_auroras_onecloudlayer" :`true` "/Game/DynamicSky/Materials/Ultra_Dynamic_Sky_Mat_onecloudlayer.Ultra_Dynamic_Sky_Mat_onecloudlayer" :!type "MaterialInterface Object Reference"))))
  (set `self.UDM_mat` _returnvalue_2)
  (bind _returnvalue_3 (`PrimitiveComponent.CreateDynamicMaterialInstance` (`self.moon_plane`) 0 "/Game/DynamicSky/Materials/moon_material.moon_material"))
  (set `self.Moon mat` _returnvalue_3)
  (`self.Set Solar Angle`)
  (`self.Set Material Variables`)
  (`/Engine/EditorBlueprintResources/StandardMacros.IsValid` _skylight
    (:`Is Valid`
      (if (`self.Use Fast Skylight`)
        (`SkyLightComponent.SetCubemap` (`SkyLight.LightComponent` (`self.Skylight`)) "/Game/DynamicSky/Textures/flat.flat")
        (else
          (`SkyLightComponent.RecaptureSky` (`SkyLight.LightComponent` _skylight)))))))