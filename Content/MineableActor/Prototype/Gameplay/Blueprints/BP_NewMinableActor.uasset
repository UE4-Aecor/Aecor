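; Prototype mineable actor that loses durability while the player mines it.
; Interact moves a spark effect to the hit point, shows it and toggles a gate that lets Tick decrement Durability every frame, hiding the sparks when it reaches zero.
; A timeline sweep that pulls the actor into the player, shrinks it, shows a notification and destroys it is present but disconnected, so never runs.
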(event `self.ReceiveTick`
  (params (DeltaSeconds :type "Float (single-precision)"))
  (bind _durability (`self.Durability`))
  ;[1 1 1] Actor Tick
  (`/Engine/EditorBlueprintResources/StandardMacros.Gate` true :!label _label
    (:`Exit`
      ;;[1 1 1] Branch will fire only once
      (`/Engine/EditorBlueprintResources/StandardMacros.DecrementInt` _durability
        (:`  `
          (if (== _durability 0)
            (`SceneComponent.SetVisibility` (`self.Sparks`) false false)))))))

(event `/Game/MineableActor/Prototype/Gameplay/Blueprints/BP_InteractionInterface.Interact`
  (params (HeadsUpDisplay :type "/Game/CompassInteraction/UI/Blueprints/BP_HeadsUpDisplay_PROTNew Object Reference") (HitPoint :type "Vector Structure"))
  (bind _sparks (`self.Sparks`))
  ;[1 1 1] Actor Tick
  (bind _asbp_player_character_prot (cast `/Game/StarterContent/Player/Blueprints/BP_PlayerCharacter_PROT` (`GameplayStatics.GetPlayerCharacter` 0)))
  (`SceneComponent.K2_SetWorldLocation` _sparks HitPoint false false)
  (`SceneComponent.SetVisibility` _sparks true false)
  (goto _label :!via `Toggle`))

(event `/Game/MineableActor/Prototype/Gameplay/Blueprints/BP_InteractionInterface.Hover`
  (params (HeadsUpDisplay :type "/Game/CompassInteraction/UI/Blueprints/BP_HeadsUpDisplay_PROTNew Object Reference"))
  ;[1 1 1] Hover Parent Function
  (`parent.Hover` HeadsUpDisplay))

(fn `UserConstructionScript`
  (`parent.UserConstructionScript`))