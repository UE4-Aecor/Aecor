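; Prototype first-person player character with walk, sprint, toggle crouch speed, jump, mouse look and a gun attached to the hands.
; Creates the HUD on BeginPlay.
; Unless interaction is disabled, Tick traces from the camera and updates compass yaw, sending hover messages to old and new targets when the hit actor changes.
; Interact press and release both message the traced actor with the HUD and hit point.
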(event `InputAxis|MoveForward`
  (params (AxisValue :type "Float (single-precision)"))
  ;[1 1 1] Base
  ;;[1 1 1] Movement
  (if (not (`self.MovementDisabled`))
    (`self.AddMovementInput` (`self.GetActorForwardVector`) AxisValue)))

(event `InputAxis|MoveRight`
  (params (AxisValue :type "Float (single-precision)"))
  ;[1 1 1] Base
  ;;[1 1 1] Movement
  (if (not (`self.MovementDisabled`))
    (`self.AddMovementInput` (`self.GetActorRightVector`) AxisValue)))

(event `InputAxis|LookUp`
  (params (AxisValue :type "Float (single-precision)"))
  ;[1 1 1] Base
  ;;[1 1 1] Looking
  (if (not (`self.LookingDisabled`))
    (`self.AddControllerPitchInput` (* AxisValue (`self.MouseSensitivity`)))))

(event `InputAxis|Turn`
  (params (AxisValue :type "Float (single-precision)"))
  ;[1 1 1] Base
  ;;[1 1 1] Looking
  (if (not (`self.LookingDisabled`))
    (`self.AddControllerYawInput` (* AxisValue (`self.MouseSensitivity`)))))

(event `InputAction|Run`
  (params (Key :type "Key Structure"))
  (bind _charactermovement (`self.CharacterMovement`))
  ;[1 1 1] Actions
  ;;[1 1 1] Running
  (:`Pressed`
    (set `self.RunPressed` true)
    (set `CharacterMovementComponent.MaxWalkSpeed` 375.0 _charactermovement))
  (:`Released`
    (set `self.RunPressed` false)
    (if (`self.CrouchPressed`)
      (set `CharacterMovementComponent.MaxWalkSpeed` 160.0 _charactermovement)
      (else
        (set `CharacterMovementComponent.MaxWalkSpeed` 200.0 _charactermovement)))))

(event `self.ReceiveBeginPlay`
  ;[1 1 1] Creating and adding HUD widget to player screen
  (bind _returnvalue (`|CreateWidget` "/Game/Prototype/UI/Blueprints/BP_HeadsUpDisplay_PROT.BP_HeadsUpDisplay_PROT_C"))
  (bind _output_get (set `self.HeadsUpDisplay` _returnvalue))
  (`UserWidget.AddToViewport` _output_get 0))

(event `InputAction|Interact`
  (params (Key :type "Key Structure"))
  ;[1 1 1] Interact
  (:`Pressed`
    (message `/Game/Prototype/Gameplay/Blueprints/BP_InteractionInterface.Interact` (`self.TraceActor`) (`self.HeadsUpDisplay`) (`self.HitPoint`) :!label _label))
  (:`Released`
    (goto _label)))

(event `InputAction|Crouch`
  (params (Key :type "Key Structure"))
  (bind _charactermovement (`self.CharacterMovement`))
  ;[1 1 1] Actions
  ;;[1 1 1] Crouching
  (:`Pressed`
    (`/Engine/EditorBlueprintResources/StandardMacros.FlipFlop`
      (:`A`
        (set `self.CrouchPressed` true)
        (set `CharacterMovementComponent.MaxWalkSpeed` 160.0 _charactermovement))
      (:`B`
        (set `self.CrouchPressed` false)
        (if (`self.RunPressed`)
          (set `CharacterMovementComponent.MaxWalkSpeed` 375.0 _charactermovement)
          (else
            (set `CharacterMovementComponent.MaxWalkSpeed` 200.0 _charactermovement)))))))

(event `InputAction|Jump`
  (params (Key :type "Key Structure"))
  ;[1 1 1] Actions
  ;;[1 1 1] Jumping
  (:`Pressed`
    (if (not (`self.MovementDisabled`))
      (`self.Jump`)
      (set `self.JumpPressed` true)))
  (:`Released`
    (set `self.JumpPressed` false)))

(event `self.ReceiveTick`
  (params (DeltaSeconds :type "Float (single-precision)"))
  (bind (_returnvalue_roll _returnvalue_pitch _returnvalue_yaw) (`KismetMathLibrary.BreakRotator` (`self.K2_GetActorRotation`)))
  ;[1 1 1] Line Tracing
  (if (not (`self.InteractionDisabled`))
    (`self.LineTrace`) ; Line trace optimization
    (set `self.CompassRotation` _returnvalue_yaw)))

(fn `LineTrace`
  (bind _camera (`self.Camera`))
  (bind _traceactor (`self.TraceActor`))
  (bind _headsupdisplay (`self.HeadsUpDisplay`))
  (bind _returnvalue (`SceneComponent.K2_GetComponentLocation` _camera))
  (bind _outhit (`KismetSystemLibrary.LineTraceSingle` _returnvalue (+ _returnvalue (* (`KismetMathLibrary.GetForwardVector` (`SceneComponent.K2_GetComponentRotation` _camera)) (`self.InteractionDistance`))) "TraceTypeQuery1"))
  (bind (_bblockinghit _binitialoverlap _time _distance _location _impactpoint _normal _impactnormal _physmat _hitactor) (`GameplayStatics.BreakHitResult` _outhit))
  (set `self.HitPoint` _impactpoint)
  (if (!= _traceactor _hitactor)
    (message `/Game/Prototype/Gameplay/Blueprints/BP_InteractionInterface.Hover` _traceactor _headsupdisplay)
    (bind _output_get (set `self.TraceActor` _hitactor))
    (message `/Game/Prototype/Gameplay/Blueprints/BP_InteractionInterface.Hover` _output_get _headsupdisplay)))

(fn `SetLaserVisibility`
  (params (Visibility :type Boolean))
  (`SceneComponent.SetVisibility` (`self.Laser`) Visibility false))

(fn `UserConstructionScript`
  (`SceneComponent.K2_AttachToComponent` (`self.Gun`) (`self.Hands`) "GripPoint" "SnapToTarget" "SnapToTarget" "SnapToTarget" true))