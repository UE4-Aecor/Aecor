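; Mineable prototype actor that the player drains with a laser, then collects.
; Interact shows the player's laser and sparks at the hit point and toggles a gate that lets Tick decrement Durability each frame.
; At zero, it hides both effects and plays a timeline that pulls the actor toward the player pawn while shrinking its mesh.
; When the timeline finishes, it shows a HUD notification and destroys itself.
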(event `self.ReceiveTick`
  (params (DeltaSeconds :type "Float (single-precision)"))
  (bind _durability (`self.Durability`))
  ;[1 1 1] Actor Tick
  (`/Engine/EditorBlueprintResources/StandardMacros.Gate` true :!label _label
    (:`Exit`
      ;;[1 1 1] Branch will fire only once
      (`/Engine/EditorBlueprintResources/StandardMacros.DecrementInt` _durability
        (:`  `
          (if (== _durability 0)
            (`SceneComponent.SetVisibility` (`self.Sparks`) false false)
            (`/Game/Prototype/Characters/Player/Blueprints/BP_PlayerCharacter_PROT.SetLaserVisibility` (stale `/Game/Prototype/Gameplay/Blueprints/BP_InteractionInterface.Interact` _asbp_player_character_prot) false)
            (bind _output_get (set `self.ActorStartLocation` (`self.K2_GetActorLocation`)))
            (bind (_direction _alpha) (`Timeline|SweepAnimation` :!via `PlayFromStart`)
              (:`Update`
                ;;[1 1 1] Sweep Animation Update
                (`self.K2_SetActorLocation` (`KismetMathLibrary.VLerp` _output_get (`self.K2_GetActorLocation` (`GameplayStatics.GetPlayerPawn` 0)) _alpha))
                (`SceneComponent.SetWorldScale3D` (`self.StaticMesh`) (`KismetMathLibrary.VLerp` (1.0 1.0 1.0) (0.0 0.0 0.0) _alpha)))
              (:`Finished`
                ;[1 1 1] Sweep Animation Finished
                (`/Game/Prototype/UI/Blueprints/BP_HeadsUpDisplay_PROT.ShowNotification` (stale `/Game/Prototype/Gameplay/Blueprints/BP_InteractionInterface.Interact` HeadsUpDisplay))
                (`self.K2_DestroyActor`)))))))))

(event `/Game/Prototype/Gameplay/Blueprints/BP_InteractionInterface.Interact`
  (params (HeadsUpDisplay :type "/Game/Prototype/UI/Blueprints/BP_HeadsUpDisplay_PROT Object Reference") (HitPoint :type "Vector Structure"))
  (bind _sparks (`self.Sparks`))
  ;[1 1 1] Actor Tick
  (bind _asbp_player_character_prot (cast `/Game/Prototype/Characters/Player/Blueprints/BP_PlayerCharacter_PROT` (`GameplayStatics.GetPlayerCharacter` 0)))
  (`/Game/Prototype/Characters/Player/Blueprints/BP_PlayerCharacter_PROT.SetLaserVisibility` _asbp_player_character_prot true)
  (`SceneComponent.K2_SetWorldLocation` _sparks HitPoint false false)
  (`SceneComponent.SetVisibility` _sparks true false)
  (goto _label :!via `Toggle`))

(event `/Game/Prototype/Gameplay/Blueprints/BP_InteractionInterface.Hover`
  (params (HeadsUpDisplay :type "/Game/Prototype/UI/Blueprints/BP_HeadsUpDisplay_PROT Object Reference"))
  ;[1 1 1] Hover Parent Function
  (`parent.Hover` HeadsUpDisplay))

(fn `UserConstructionScript`
  (`parent.UserConstructionScript`))