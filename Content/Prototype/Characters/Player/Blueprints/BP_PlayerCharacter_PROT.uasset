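; Prototype player character Blueprint that handles walking, mouse look, running, crouching and jumping, with a gun held in the hands.
; Movement and look axes are gated by disable flags, and look input is scaled by mouse sensitivity.
; Hold-to-run and FlipFlop-toggled crouch only change max walk speed, checking each other's state to restore it.
; The construction script snaps the Gun to the GripPoint socket on Hands.
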(event `InputAxis|MoveForward`
  (params (AxisValue :type "Float (single-precision)"))
  ;[1 1 1] Base
  ;;[1 1 1] Movement
  (if (not (`self.MovementDisabled`))
    (`self.AddMovementInput` (`self.GetActorForwardVector`) AxisValue)))

(event `InputAxis|MoveRight`
  (params (AxisValue :type "Float (single-precision)"))
  ;[1 1 1] Base
  ;;[1 1 1] Movement
  (if (not (`self.MovementDisabled`))
    (`self.AddMovementInput` (`self.GetActorRightVector`) AxisValue)))

(event `InputAxis|LookUp`
  (params (AxisValue :type "Float (single-precision)"))
  ;[1 1 1] Base
  ;;[1 1 1] Looking
  (if (not (`self.LookingDisabled`))
    (`self.AddControllerPitchInput` (* AxisValue (`self.MouseSensitivity`)))))

(event `InputAxis|Turn`
  (params (AxisValue :type "Float (single-precision)"))
  ;[1 1 1] Base
  ;;[1 1 1] Looking
  (if (not (`self.LookingDisabled`))
    (`self.AddControllerYawInput` (* AxisValue (`self.MouseSensitivity`)))))

(event `InputAction|Run`
  (params (Key :type "Key Structure"))
  (bind _charactermovement (`self.CharacterMovement`))
  ;[1 1 1] Actions
  ;;[1 1 1] Running
  (:`Pressed`
    (set `self.RunPressed` true)
    (set `CharacterMovementComponent.MaxWalkSpeed` 375.0 _charactermovement))
  (:`Released`
    (set `self.RunPressed` false)
    (if (`self.CrouchPressed`)
      (set `CharacterMovementComponent.MaxWalkSpeed` 160.0 _charactermovement)
      (else
        (set `CharacterMovementComponent.MaxWalkSpeed` 200.0 _charactermovement)))))

(event `InputAction|Crouch`
  (params (Key :type "Key Structure"))
  (bind _charactermovement (`self.CharacterMovement`))
  ;[1 1 1] Actions
  ;;[1 1 1] Crouching
  (:`Pressed`
    (`/Engine/EditorBlueprintResources/StandardMacros.FlipFlop`
      (:`A`
        (set `self.CrouchPressed` true)
        (set `CharacterMovementComponent.MaxWalkSpeed` 160.0 _charactermovement))
      (:`B`
        (set `self.CrouchPressed` false)
        (if (`self.RunPressed`)
          (set `CharacterMovementComponent.MaxWalkSpeed` 375.0 _charactermovement)
          (else
            (set `CharacterMovementComponent.MaxWalkSpeed` 200.0 _charactermovement)))))))

(event `InputAction|Jump`
  (params (Key :type "Key Structure"))
  ;[1 1 1] Actions
  ;;[1 1 1] Jumping
  (:`Pressed`
    (if (not (`self.MovementDisabled`))
      (`self.Jump`)
      (set `self.JumpPressed` true)))
  (:`Released`
    (set `self.JumpPressed` false)))

(fn `UserConstructionScript`
  (`SceneComponent.K2_AttachToComponent` (`self.Gun`) (`self.Hands`) "GripPoint" "SnapToTarget" "SnapToTarget" "SnapToTarget" true))